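; Player controller for a tank game that sets up the player HUD and handles opening the pause menu.
; When FoundAimingComponent fires, it creates the player UI widget, adds it to the viewport and passes it the aiming component reference.
; The Quit input lazily creates and caches the pause menu, shows it with UI-only input and a mouse cursor, and pauses the game.
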(event EventBeginPlay)

(event EventFoundAimingComponent
  (params (AimCompRef :type Tank%20Aiming%20Component%20Object%20Reference))
  (bind _returnvalue (UserInterface|CreateWidget "/Game/UI/PlayerUI_BP.PlayerUI_BP_C"))
  (bind _output_get (Variables|Default|SetHUD%20reference _returnvalue))
  (UserInterface|Viewport|AddtoViewport _output_get 0)
  (Variables|/Game/UI/PlayerUI_BP.PlayerUI_BP_C|SetBP%20Aiming%20Comp%20Reference _output_get AimCompRef))

(event EventTick
  (params (DeltaSeconds :type Float%20%28single-precision%29)))

(event Input|ActionEvents|InputActionQuit
  (params (Key :type Key%20Structure))
  ;[1 1 1] Pause menu
  (:Pressed
    (Utilities|IsValid (Variables|Default|GetPause%20Menu%20Reference)
      (:Is%20Valid
        _)
      (:Is%20Not%20Valid
        (bind _returnvalue (UserInterface|CreateWidget "/Game/UI/PauseMenu_BP.PauseMenu_BP_C"))
        (bind _output_get (Variables|Default|SetPause%20Menu%20Reference _returnvalue))))
    (Input|SetInputModeUIOnly (Game|GetPlayerController 0) _output_get "DoNotLock")
    (UserInterface|Viewport|AddtoViewport (Variables|Default|GetPause%20Menu%20Reference) 0)
    (Game|SetGamePaused true)
    (Variables|Default|SetbShowMouseCursor true)))

(fn ConstructionScript)